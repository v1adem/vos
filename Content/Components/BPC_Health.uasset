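; BPC_Health is a health component that tracks current and maximum health for its owner.
; On BeginPlay it fills current health to the maximum.
; Functions add or subtract health, clamped at the maximum and at zero respectively, and report the current value or whether it has reached zero.
; It has no death event or change notification, so other code reads the state through GetHealth and IsDead.
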(event EventBeginPlay
  (CallFunction|SetMaxHealth))

(event EventTick
  (params (DeltaSeconds :type Float%20%28single-precision%29)))

(fn GetHealth
  (return (Variables|Default|GetCurrentHealth)))

(fn IsDead
  (return (<= (Variables|Default|GetCurrentHealth) 0.0)))

(fn AddHealth
  (params (Heal :type Float%20%28double-precision%29))
  (Variables|Default|SetCurrentHealth (Math|Float|Min(Float) (+ Heal (Variables|Default|GetCurrentHealth)) (Variables|Default|GetMaxHealth)))
  (return))

(fn SubtractHealth
  (params (Damage :type Float%20%28double-precision%29))
  (Variables|Default|SetCurrentHealth (Math|Float|Max(Float) (- (Variables|Default|GetCurrentHealth) Damage) 0.0))
  (return))

(fn SetMaxHealth
  (Variables|Default|SetCurrentHealth (Variables|Default|GetMaxHealth))
  (return))